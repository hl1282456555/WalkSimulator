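; BP_TCPMonitor is a VR monitor pawn that links to a TCP server, mirroring server-side walkers and reporting the player's state.
; Received bytes are buffered as a string; each tick extracts one @@…## framed JSON message, then spawns, moves or destroys BP_TCPWalker actors by ID.
; It also sends camera transform and motion controller inputs as framed JSON every tick.
; R teleports the HMD to the game mode's default transform.
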(event EventBeginPlay
  (bind _returnvalue (Game|SpawnActorfromClass "/Script/TcpSocketPlugin.TcpSocketConnection" (Math|Transform|MakeTransform "0, 0, 0") "AlwaysSpawn" 0 0))
  (Variables|Default|SetTCPSocketConnectorRef _returnvalue)
  (bind _connectionid (Class|TcpSocketConnection|Connect (Variables|Default|GetTCPSocketConnectorRef) (Variables|Default|GetTCPServerIP) (Variables|Default|GetTCPServerPort) (EventDispatchers|CreateEvent :!event BPTCPMonitorDisconnectedCallback) (EventDispatchers|CreateEvent :!event BPTCPMonitorConnectedCallback) (EventDispatchers|CreateEvent :!event BPTCPMonitorReceivedCallback)))
  (Variables|Default|SetHandlerId _connectionid)
  (bind _asbp_tcpgame_mode (Utilities|Casting|CastToBP_TCPGameMode (Game|GetGameMode)))
  (Variables|Default|SetGameModeRef _asbp_tcpgame_mode)
  (Input|EnableInput (Game|GetPlayerController 0))
  (Class|HeadMountedDisplayFunctionLibrary|SetTrackingOrigin "Floor"))

(event EventEndPlay
  (params (EndPlayReason :type EEndPlayReason%20Enum :default "Destroyed"))
  (CallFunction|ClearWalker)
  (Utilities|IsValid (Variables|Default|GetTCPSocketConnectorRef)
    (:Is%20Valid
      (Class|TcpSocketConnection|Disconnect (Variables|Default|GetTCPSocketConnectorRef) (Variables|Default|GetHandlerId)))))

(event EventTick
  (params (DeltaSeconds :type Float%20%28single-precision%29))
  (bind _message (CallFunction|PrepareNextMessage))
  (CallFunction|ProcessMessage _message)
  (CallFunction|SendCurrentStatetoServer))

(event Input|ActionEvents|InputActionLeftTrackRight
  (params (Key :type Key%20Structure :default "None"))
  (:Pressed
    (Variables|Default|SetLeftTrackRight true))
  (:Released
    (Variables|Default|SetLeftTrackRight false)))

(event Input|ActionEvents|InputActionLeftTrackLeft
  (params (Key :type Key%20Structure :default "None"))
  (:Pressed
    (Variables|Default|SetLeftTrackLeft true))
  (:Released
    (Variables|Default|SetLeftTrackLeft false)))

(event Input|ActionEvents|InputActionLeftTrackUp
  (params (Key :type Key%20Structure :default "None"))
  (:Pressed
    (Variables|Default|SetLeftTrackUp true))
  (:Released
    (Variables|Default|SetLeftTrackUp false)))

(event Input|ActionEvents|InputActionLeftTrackDown
  (params (Key :type Key%20Structure :default "None"))
  (:Pressed
    (Variables|Default|SetLeftTrackDown true))
  (:Released
    (Variables|Default|SetLeftTrackDown false)))

(event Input|ActionEvents|InputActionLeftGrip
  (params (Key :type Key%20Structure :default "None"))
  (:Pressed
    (Variables|Default|SetLeftGrip true))
  (:Released
    (Variables|Default|SetLeftGrip false)))

(event Input|ActionEvents|InputActionRightTrackLeft
  (params (Key :type Key%20Structure :default "None"))
  (:Pressed
    (Variables|Default|SetRightTrackLeft true))
  (:Released
    (Variables|Default|SetRightTrackLeft false)))

(event Input|ActionEvents|InputActionRightTrackRight
  (params (Key :type Key%20Structure :default "None"))
  (:Pressed
    (Variables|Default|SetRightTrackRight true))
  (:Released
    (Variables|Default|SetRightTrackRight false)))

(event Input|ActionEvents|InputActionRightTrackUp
  (params (Key :type Key%20Structure :default "None"))
  (:Pressed
    (Variables|Default|SetRightTrackUp true))
  (:Released
    (Variables|Default|SetRightTrackUp false)))

(event Input|ActionEvents|InputActionRightTrackDown
  (params (Key :type Key%20Structure :default "None"))
  (:Pressed
    (Variables|Default|SetRightTrackDown true))
  (:Released
    (Variables|Default|SetRightTrackDown false)))

(event Input|ActionEvents|InputActionRightGrip
  (params (Key :type Key%20Structure :default "None"))
  (:Pressed
    (Variables|Default|SetRightGrip true))
  (:Released
    (Variables|Default|SetRightGrip false)))

(event Input|AxisEvents|InputAxisLeftTrigger
  (params (AxisValue :type Float%20%28single-precision%29))
  (Variables|Default|SetLeftTriggerAxis AxisValue))

(event Input|AxisEvents|InputAxisRightTrigger
  (params (AxisValue :type Float%20%28single-precision%29))
  (Variables|Default|SetRightTriggerAxis AxisValue))

(event Input|KeyboardEvents|R
  (params (Key :type Key%20Structure :default "None"))
  (bind _gamemoderef (Variables|Default|GetGameModeRef))
  (bind _monitordefaulttransform (Variables|/Game/Blueprints/TCP/BP_TCPGameMode.BP_TCPGameMode_C|GetMonitorDefaultTransform _gamemoderef))
  (:Pressed
    (Transformation|Teleport (- (.location _monitordefaulttransform) (Math|Vector|RotateVector (.DevicePosition (Class|HeadMountedDisplayFunctionLibrary|GetOrientationandPosition)) (.rotation _monitordefaulttransform))) (.rotation _monitordefaulttransform))
    (Class|HeadMountedDisplayFunctionLibrary|ResetOrientationandPosition 0.0 "Orientation")))

(fn ConstructionScript)

(fn BPTCPMonitorDisconnectedCallback
  (params (ConnectionId :type Integer)))

(fn BPTCPMonitorConnectedCallback
  (params (ConnectionId :type Integer))
  (Development|PrintString (Utilities|String|Append "Connect to tcp server succeeded, handle id : " (Utilities|String|ToString(Integer) ConnectionId)) false))

(fn BPTCPMonitorReceivedCallback
  (params (ConnectionId :type Integer) (Message :type Array%20of%20Bytes))
  (if (== ConnectionId (Variables|Default|GetHandlerId))
    (bind _returnvalue (Class|TcpSocketConnection|MessageReadString (Variables|Default|GetTCPSocketConnectorRef) Message (Utilities|Array|Length Message)))
    (Variables|Default|SetCachedMessage (Utilities|String|Append (Variables|Default|GetCachedMessage) _returnvalue))))

(fn PrepareNextMessage
  (if (Utilities|String|StartsWith (Variables|Default|GetCachedMessage) "@@")
    (LocalVariables|SetLocalFoundIndex (Utilities|String|FindSubstring (Variables|Default|GetCachedMessage) "##"))
    (if (!= (LocalVariables|GetLocalFoundIndex) -1)
      (LocalVariables|SetLocalParseMessage (Utilities|String|GetSubstring (Variables|Default|GetCachedMessage) 0 (+ (LocalVariables|GetLocalFoundIndex) 2)))
      (Variables|Default|SetCachedMessage (Utilities|String|GetSubstring (Variables|Default|GetCachedMessage) (+ (LocalVariables|GetLocalFoundIndex) 2) (- (Utilities|String|Len (Variables|Default|GetCachedMessage)) (+ (LocalVariables|GetLocalFoundIndex) 2))))
      (return (LocalVariables|GetLocalParseMessage)))))

(fn ProcessMessage
  (params (Message :type String))
  (if (not (Utilities|Array|IsEmpty Message))
    (LocalVariables|SetLocalParsedJson (.RightS (Utilities|String|Split Message "@@")))
    (LocalVariables|SetLocalParsedJson (.LeftS (Utilities|String|Split (LocalVariables|GetLocalParsedJson) "##" "IgnoreCase" "FromEnd")))
    (bind _returnvalue (Class|VaRestSubsystem|ConstructVaRestJsonObject (|VaRestSubsystem)))
    (LocalVariables|SetLocalServerJson _returnvalue)
    (bind _returnvalue_2 (Class|VaRestJsonObject|DecodeJson (LocalVariables|GetLocalServerJson) (LocalVariables|GetLocalParsedJson) true))
    (if _returnvalue_2
      (LocalVariables|SetLocalWalkerList (Class|VaRestJsonObject|GetObjectArrayField (LocalVariables|GetLocalServerJson) "walkerList"))
      (for _array_element (LocalVariables|GetLocalWalkerList)
        (LocalVariables|SetLocalCurrentWalkerJson _array_element)
        (LocalVariables|SetLocalCurrentWalkerId (Class|VaRestJsonObject|GetIntegerField (LocalVariables|GetLocalCurrentWalkerJson) "walkerId"))
        (LocalVariables|SetLocalNewLocation (Math|Vector|MakeVector (Class|VaRestJsonObject|GetNumberField (LocalVariables|GetLocalCurrentWalkerJson) "locationX") (Class|VaRestJsonObject|GetNumberField (LocalVariables|GetLocalCurrentWalkerJson) "locationY") (Class|VaRestJsonObject|GetNumberField (LocalVariables|GetLocalCurrentWalkerJson) "locationZ")))
        (if (.ReturnValue (Utilities|Map|Find (Variables|Default|GetTCPWalkerMap) (LocalVariables|GetLocalCurrentWalkerId)))
          (LocalVariables|SetLocalCurrentWalkerRef (.Value (Utilities|Map|Find (Variables|Default|GetTCPWalkerMap) (LocalVariables|GetLocalCurrentWalkerId))))
          (Default|ProcessNewLocation (LocalVariables|GetLocalCurrentWalkerRef) (LocalVariables|GetLocalNewLocation))
          (Utilities|Array|Add (LocalVariables|GetLocalServerWalkerList) (LocalVariables|GetLocalCurrentWalkerId))
          (else
            (bind _returnvalue_3 (Game|SpawnActorfromClass "/Game/Blueprints/TCP/BP_TCPWalker.BP_TCPWalker_C" (Math|Transform|MakeTransform (LocalVariables|GetLocalNewLocation)) "AlwaysSpawn" 0 0))
            (Utilities|Map|Add (Variables|Default|GetTCPWalkerMap) (LocalVariables|GetLocalCurrentWalkerId) _returnvalue_3)
            (Utilities|Array|Add (LocalVariables|GetLocalServerWalkerList) (LocalVariables|GetLocalCurrentWalkerId)))))
      (bind _keys (Utilities|Map|Keys (Variables|Default|GetTCPWalkerMap)))
      (LocalVariables|SetLocalClientWalkerList _keys)
      (for _array_element_2 (LocalVariables|GetLocalClientWalkerList)
        (LocalVariables|SetLocalCurrentWalkerId _array_element_2)
        (if (not (Utilities|Array|ContainsItem (LocalVariables|GetLocalServerWalkerList) (LocalVariables|GetLocalCurrentWalkerId)))
          (Actor|DestroyActor (.Value (Utilities|Map|Find (Variables|Default|GetTCPWalkerMap) (LocalVariables|GetLocalCurrentWalkerId))))
          (Utilities|Map|Remove (Variables|Default|GetTCPWalkerMap) (LocalVariables|GetLocalCurrentWalkerId)))))))

(fn SendCurrentStatetoServer
  (bind _camera (Variables|Default|GetCamera))
  (bind _camera_2 (Variables|Default|GetCamera))
  (bind _returnvalue (Transformation|GetWorldLocation _camera_2))
  (bind _returnvalue_2 (Transformation|GetWorldRotation _camera))
  (Utilities|IsValid (Variables|Default|GetTCPSocketConnectorRef)
    (:Is%20Valid
      (if (Class|TcpSocketConnection|IsConnected (Variables|Default|GetTCPSocketConnectorRef) (Variables|Default|GetHandlerId))
        (bind _returnvalue_3 (Class|VaRestSubsystem|ConstructVaRestJsonObject (|VaRestSubsystem)))
        (LocalVariables|SetLocalLeftMCJson _returnvalue_3)
        (bind _returnvalue_4 (Class|VaRestSubsystem|ConstructVaRestJsonObject (|VaRestSubsystem)))
        (LocalVariables|SetLocalRightMCJson _returnvalue_4)
        (bind _returnvalue_5 (Class|VaRestSubsystem|ConstructVaRestJsonObject (|VaRestSubsystem)))
        (LocalVariables|SetLocalPlayerTJson _returnvalue_5)
        (bind _returnvalue_6 (Class|VaRestSubsystem|ConstructVaRestJsonObject (|VaRestSubsystem)))
        (LocalVariables|SetLocalClientStateJson _returnvalue_6)
        (Class|VaRestJsonObject|SetBoolField (LocalVariables|GetLocalLeftMCJson) "TrackLeft" (Variables|Default|GetLeftTrackLeft))
        (Class|VaRestJsonObject|SetBoolField (LocalVariables|GetLocalLeftMCJson) "TrackRight" (Variables|Default|GetLeftTrackRight))
        (Class|VaRestJsonObject|SetBoolField (LocalVariables|GetLocalLeftMCJson) "TrackUp" (Variables|Default|GetLeftTrackUp))
        (Class|VaRestJsonObject|SetBoolField (LocalVariables|GetLocalLeftMCJson) "TrackDown" (Variables|Default|GetLeftTrackDown))
        (Class|VaRestJsonObject|SetBoolField (LocalVariables|GetLocalLeftMCJson) "trigger" (!= (Variables|Default|GetLeftTriggerAxis) 0.0))
        (Class|VaRestJsonObject|SetBoolField (LocalVariables|GetLocalLeftMCJson) "gripButton" (Variables|Default|GetLeftGrip))
        (Class|VaRestJsonObject|SetBoolField (LocalVariables|GetLocalRightMCJson) "TrackLeft" (Variables|Default|GetRightTrackLeft))
        (Class|VaRestJsonObject|SetBoolField (LocalVariables|GetLocalRightMCJson) "TrackRight" (Variables|Default|GetRightTrackRight))
        (Class|VaRestJsonObject|SetBoolField (LocalVariables|GetLocalRightMCJson) "TrackUp" (Variables|Default|GetRightTrackUp))
        (Class|VaRestJsonObject|SetBoolField (LocalVariables|GetLocalRightMCJson) "TrackDown" (Variables|Default|GetRightTrackDown))
        (Class|VaRestJsonObject|SetBoolField (LocalVariables|GetLocalRightMCJson) "trigger" (!= (Variables|Default|GetRightTriggerAxis) 0.0))
        (Class|VaRestJsonObject|SetBoolField (LocalVariables|GetLocalRightMCJson) "gripButton" (Variables|Default|GetRightGrip))
        (Class|VaRestJsonObject|SetNumberField (LocalVariables|GetLocalPlayerTJson) "locationX" (.x _returnvalue))
        (Class|VaRestJsonObject|SetNumberField (LocalVariables|GetLocalPlayerTJson) "locationY" (.y _returnvalue))
        (Class|VaRestJsonObject|SetNumberField (LocalVariables|GetLocalPlayerTJson) "locationZ" (.z _returnvalue))
        (Class|VaRestJsonObject|SetNumberField (LocalVariables|GetLocalPlayerTJson) "roll" (.roll _returnvalue_2))
        (Class|VaRestJsonObject|SetNumberField (LocalVariables|GetLocalPlayerTJson) "pitch" (.pitch _returnvalue_2))
        (Class|VaRestJsonObject|SetNumberField (LocalVariables|GetLocalPlayerTJson) "yaw" (.yaw _returnvalue_2))
        (Class|VaRestJsonObject|SetObjectField (LocalVariables|GetLocalClientStateJson) "leftMotionController" (LocalVariables|GetLocalLeftMCJson))
        (Class|VaRestJsonObject|SetObjectField (LocalVariables|GetLocalClientStateJson) "rightMotionController" (LocalVariables|GetLocalRightMCJson))
        (Class|VaRestJsonObject|SetObjectField (LocalVariables|GetLocalClientStateJson) "playerTransfrom" (LocalVariables|GetLocalPlayerTJson))
        (LocalVariables|SetLocalClientStateJsonStr (Utilities|String|Append "@@" (Class|VaRestJsonObject|EncodeJsontoSingleString (LocalVariables|GetLocalClientStateJson)) "##"))
        (bind _returnvalue_7 (Class|TcpSocketConnection|SendData (Variables|Default|GetTCPSocketConnectorRef) (Variables|Default|GetHandlerId) (Class|TcpSocketConnection|ToBytes(String) (Variables|Default|GetTCPSocketConnectorRef) (LocalVariables|GetLocalClientStateJsonStr))))
        (Development|PrintString (Utilities|String|Append "Send data to server " (Utilities|String|ToString(Boolean) _returnvalue_7)) false)))))

(fn ClearWalker
  (bind _values (Utilities|Map|Values (Variables|Default|GetTCPWalkerMap)))
  (Actor|DestroyActor _values)
  (Utilities|Map|Clear (Variables|Default|GetTCPWalkerMap)))