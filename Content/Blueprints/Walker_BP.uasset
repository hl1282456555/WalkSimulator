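; Walker pedestrian for a walk simulation with data capture, dressed in a random character at BeginPlay.
; It takes a unique name from the GameState pool, loads mesh and AnimClass from a DataTable, and returns the name when hidden.
; While capture state is None or Pending Capture Data, Tick drives the time-based transform and anim frame capture.
; WalkerInCameraView tests visibility with pelvis and head line traces to the player pawn.
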(event EventBeginPlay
  (bind _aswalk_simulator_gs (Utilities|Casting|CastToWalkSimulator_GS (Game|GetGameState)))
  (Variables|Default|SetGameStateRef _aswalk_simulator_gs)
  (bind _aswalk_simulator_gm (Utilities|Casting|CastToWalkSimulator_GM (Game|GetGameMode)))
  (Variables|Default|SetGameModeRef _aswalk_simulator_gm)
  (CallFunction|ChangeMesh))

(event Collision|EventActorBeginOverlap
  (params (OtherActor :type Actor%20Object%20Reference)))

(event EventTick
  (params (DeltaSeconds :type Float%20%28single-precision%29))
  (bind _gamestateref (Variables|Default|GetGameStateRef))
  (|CallParentFunction DeltaSeconds)
  (Utilities|IsValid _gamestateref
    (:Is%20Valid
      (switch Utilities|FlowControl|Switch|SwitchonECaptureState (Variables|/Game/Blueprints/WalkSimulator_GS.WalkSimulator_GS_C|GetCaptureState _gamestateref)
        (:None
          _)
        (:PendingCaptureData
          _))
      (Class|Walker|SetWalkerTransform (- (Utilities|Time|GetTimeSeconds) (Variables|Default|GetSimulateTime)))
      (Class|Walker|CaptureAnimFrame (Variables|/Script/WalkSimulator.WalkSimulatorGameModeBase|GetStartSimulateTime (Variables|Default|GetGameModeRef))))))

(event EventOnMeshHidden
  (Utilities|Array|AddUnique (Variables|/Game/Blueprints/WalkSimulator_GS.WalkSimulator_GS_C|GetCharacterMeshNames (Variables|Default|GetGameStateRef)) (Variables|Default|GetCharacterMeshName)))

(fn ConstructionScript)

(fn WalkerinCameraView
  (bind (_outhit _returnvalue) (Collision|LineTraceByChannel (Transformation|GetSocketLocation (Variables|Default|GetSkeletalMesh) "Pelvis") (Transformation|GetActorLocation (Game|Player|GetPlayerPawn 0)) "TraceTypeQuery1" true 0 "None"))
  (if _returnvalue
    (if (== (.HitActor (Collision|BreakHitResult _outhit)) (Game|Player|GetPlayerPawn 0))
      (return true)
      (else
        _)))
  (bind (_outhit_2 _returnvalue_2) (Collision|LineTraceByChannel (Transformation|GetSocketLocation (Variables|Default|GetSkeletalMesh) "head") (Transformation|GetActorLocation (Game|Player|GetPlayerPawn 0)) "TraceTypeQuery1" true 0 "None"))
  (if _returnvalue_2
    (if (== (.HitActor (Collision|BreakHitResult _outhit_2)) (Game|Player|GetPlayerPawn 0))
      (return true)
      (else
        (return false)))))

(fn ChangeMesh
  (LocalVariables|SetLocal_MeshNum (Math|Random|RandomInteger (Utilities|Array|Length (Variables|/Game/Blueprints/WalkSimulator_GS.WalkSimulator_GS_C|GetCharacterMeshNames (Variables|Default|GetGameStateRef)))))
  (Variables|Default|SetCharacterMeshName (Utilities|Array|Get(acopy) (Variables|/Game/Blueprints/WalkSimulator_GS.WalkSimulator_GS_C|GetCharacterMeshNames (Variables|Default|GetGameStateRef)) (LocalVariables|GetLocal_MeshNum)))
  (Utilities|Array|RemoveItem (Variables|/Game/Blueprints/WalkSimulator_GS.WalkSimulator_GS_C|GetCharacterMeshNames (Variables|Default|GetGameStateRef)) (Variables|Default|GetCharacterMeshName))
  (bind _returnvalue (Utilities|GetDataTableRow (Variables|Default|GetCharacter_DataTable) (Variables|Default|GetCharacterMeshName))
    (:then
      (LocalVariables|SetLocal_Mesh (.SleletalMesh (Utilities|Struct|BreakCharacter_Struct _returnvalue)))
      (Class|SkeletalMeshComponent|SetAnimClass (Variables|Default|GetSkeletalMesh) (.AnimInstance (Utilities|Struct|BreakCharacter_Struct _returnvalue)))
      (Class|SkinnedMeshComponent|SetSkeletalMesh (Variables|Default|GetSkeletalMesh) (LocalVariables|GetLocal_Mesh) true)
      (Class|SkinnedMeshComponent|SetSkeletalMesh (Variables|Default|GetPoseableMesh) (LocalVariables|GetLocal_Mesh) true))))