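; BP_TCPWalker is a walker actor that moves to locations passed into it and derives its facing and speed from that motion.
; ProcessNewLocation ignores negligible moves, otherwise sets the location without sweep and yaws the actor along the direction from its previous position.
; It computes WalkerSpeed from distance over DeltaTime, then caches the transform, first stored at BeginPlay, for the next update.
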(event EventBeginPlay
  (Variables|Default|SetPreActorTransform (Transformation|GetActorTransform)))

(event Collision|EventActorBeginOverlap
  (params (OtherActor :type Actor%20Object%20Reference)))

(event EventTick
  (params (DeltaSeconds :type Float%20%28single-precision%29)))

(fn ConstructionScript)

(fn ProcessNewLocation
  (params (NewLocation :type Vector) (DeltaTime :type Float%20%28single-precision%29))
  (if (not (Math|Vector|Equal(Vector) NewLocation (Transformation|GetActorLocation) 0.01))
    (Transformation|SetActorLocation NewLocation false false)
    (LocalVariables|SetLocalRotationYaw (.yaw (Math|Rotator|FindLookatRotation (.Location (Math|Transform|BreakTransform (Variables|Default|GetPreActorTransform))) NewLocation)))
    (Transformation|SetActorRotation (Math|Rotator|MakeRotator 0.0 0.0 (LocalVariables|GetLocalRotationYaw)))
    (Variables|Default|SetWalkerSpeed (/ (Math|Float|Absolute(Float) (Math|Vector|VectorLength (- NewLocation (.Location (Math|Transform|BreakTransform (Variables|Default|GetPreActorTransform)))))) DeltaTime))
    (Variables|Default|SetPreActorTransform (Transformation|GetActorTransform))))