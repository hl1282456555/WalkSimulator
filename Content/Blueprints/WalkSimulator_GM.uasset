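; Game mode for a walk simulator that populates the level with walkers following predefined paths.
; On BeginPlay it caches the player pawn and game state, then stores the InitWalkPath result as the game state's path map, keyed by walker ID.
; It spawns a Walker_BP at each path's first point and assigns its ID and points.
; StartCaptureMovie moves the pawn through every monitor transform in one loop, without delays or capture logic.
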(event EventBeginPlay
  (bind _aswalk_simulator_pawn_bp (Utilities|Casting|CastToWalkSimulatorPawn_BP (Pawn|GetControlledPawn (Game|GetPlayerController 0))))
  (Variables|Default|SetPlayerPawnRef _aswalk_simulator_pawn_bp)
  (bind _aswalk_simulator_gs (Utilities|Casting|CastToWalkSimulator_GS (Game|GetGameState)))
  (Variables|Default|SetGameStateRef _aswalk_simulator_gs)
  (CallFunction|InitializeWalkers))

(event EventTick
  (params (DeltaSeconds :type Float%20%28single-precision%29)))

(fn ConstructionScript)

(fn StartCaptureMovie
  (for _array_element (Variables|/Game/Blueprints/WalkSimulator_GS.WalkSimulator_GS_C|GetMonitorList (Variables|Default|GetGameStateRef))
    (LocalVariables|SetLocalCurrentMonitor _array_element)
    (Transformation|SetActorTransform (Variables|Default|GetPlayerPawnRef) (Transformation|GetActorTransform (LocalVariables|GetLocalCurrentMonitor)))))

(fn InitializeWalkers
  (bind _walkpath (Class|WalkSimulatorFunctionLibrary|InitWalkPath))
  (Variables|/Game/Blueprints/WalkSimulator_GS.WalkSimulator_GS_C|SetWalkerPaths (Variables|Default|GetGameStateRef) _walkpath)
  (bind _keys (Utilities|Map|Keys (Variables|/Game/Blueprints/WalkSimulator_GS.WalkSimulator_GS_C|GetWalkerPaths (Variables|Default|GetGameStateRef))))
  (LocalVariables|SetLocalAllWalkerIds _keys)
  (for _array_element (LocalVariables|GetLocalAllWalkerIds)
    (LocalVariables|SetLocalCurrentWalkerId _array_element)
    (LocalVariables|SetLocalCurrentWalkPath (.Value (Utilities|Map|Find (Variables|/Game/Blueprints/WalkSimulator_GS.WalkSimulator_GS_C|GetWalkerPaths (Variables|Default|GetGameStateRef)) (LocalVariables|GetLocalCurrentWalkerId))))
    (bind _returnvalue (Game|SpawnActorfromClass "/Game/Blueprints/Walker_BP.Walker_BP_C" (Math|Transform|MakeTransform (Utilities|Struct|BreakPathPoint (Utilities|Array|Get(acopy) (Utilities|Struct|BreakPathPointList (LocalVariables|GetLocalCurrentWalkPath))))) "Undefined" 0 0))
    (LocalVariables|SetLocalCurrentWalker _returnvalue)
    (Variables|/Script/WalkSimulator.Walker|SetWalkerId (LocalVariables|GetLocalCurrentWalker) (LocalVariables|GetLocalCurrentWalkerId))
    (Variables|/Script/WalkSimulator.Walker|SetPathPoints (LocalVariables|GetLocalCurrentWalker) (Utilities|Struct|BreakPathPointList (LocalVariables|GetLocalCurrentWalkPath)))))