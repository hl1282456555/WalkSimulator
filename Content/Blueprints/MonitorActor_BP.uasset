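; MonitorActor_BP is a placeable surveillance camera actor that is positioned with the mouse and renders its view through a scene capture.
; On BeginPlay it names itself from an incrementing ID in WalkSimulator_GS, and on destruction it removes itself from that game state's monitor list.
; Mouse placement snaps to a visibility trace hit or floats at a fixed distance along the cursor ray.
; Toggling capture clears the render target and hides BaseGizmo actors from the camera.
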(event EventBeginPlay
  (bind _aswalk_simulator_gs (Utilities|Casting|CastToWalkSimulator_GS (Game|GetGameState)))
  (Variables|Default|SetGameStateRef _aswalk_simulator_gs)
  (Variables|Default|SetCameraName (Utilities|String|Append "监控_" (Utilities|String|ToString(Integer) (Variables|/Game/Blueprints/WalkSimulator_GS.WalkSimulator_GS_C|GetMonitorNameId (Variables|Default|GetGameStateRef)))))
  (Math|Integer|IncrementInt (Variables|/Game/Blueprints/WalkSimulator_GS.WalkSimulator_GS_C|GetMonitorNameId (Variables|Default|GetGameStateRef))))

(event EventDestroyed
  (Utilities|Array|RemoveItem (Variables|/Game/Blueprints/WalkSimulator_GS.WalkSimulator_GS_C|GetMonitorList (Variables|Default|GetGameStateRef)) self))

(fn ConstructionScript)

(fn MoveMonitorUseMouse
  (params (MousePosition :type Vector%202D%20Structure))
  (bind _returnvalue (Game|GetPlayerController 0))
  (bind _returnvalue_2 (Game|GetPlayerController 0))
  (bind (_worldposition _worlddirection) (Class|GameplayStatics|DeprojectScreentoWorld _returnvalue_2 MousePosition))
  (bind (_worldposition_2 _worlddirection_2) (Class|GameplayStatics|DeprojectScreentoWorld _returnvalue MousePosition))
  (bind _outhit (Collision|LineTraceByChannel _worldposition_2 (+ _worldposition_2 (* _worlddirection_2 1e+03)) "TraceTypeQuery1" false (Utilities|Array|MakeArray (Variables|Default|GetPlayerPawnRef)) "None"))
  (if (.bBlockingHit (Collision|BreakHitResult _outhit))
    (Transformation|SetActorLocation (.ImpactPoint (Collision|BreakHitResult _outhit)) false false)
    (else
      (Transformation|SetActorLocation (+ _worldposition (* _worlddirection 5e+02)) false false))))

(fn SetCaptureState
  (params (bShouldCapture :type Boolean))
  (Rendering|ClearRenderTarget2D "/Game/Textures/MonitorCanvas_RT.MonitorCanvas_RT")
  (Components|Activation|SetActive (Variables|Default|GetCamera) bShouldCapture true)
  (Variables|/Script/Engine.SceneCaptureComponent|SetbCaptureEveryFrame (Variables|Default|GetCamera) bShouldCapture)
  (CallFunction|UpdateGizmoHiddenList))

(fn UpdateGizmoHiddenList
  (bind _outactors (Actor|GetAllActorsOfClass "/Script/RuntimeTransformer.BaseGizmo"))
  (Variables|/Script/Engine.SceneCaptureComponent|SetHiddenActors (Variables|Default|GetCamera) _outactors))