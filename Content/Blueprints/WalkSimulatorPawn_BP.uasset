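; Free-flying camera pawn that selects and transforms objects with a runtime gizmo.
; Axis inputs offset the pawn without collision sweeps and turn the view, while Select mouse-traces two custom object channels.
; Space toggles translation in world space and rotation in local space, and Delete calls DeselectAll with its flag set.
; Selected non-UFocusable components get custom depth, and the mouse locks during gizmo drags.
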(event EventBeginPlay)

(event EventOnComponentSelectionChange
  (params (Component :type Scene%20Component%20Object%20Reference) (bSelected :type Boolean) (bImplementsUFocusable :type Boolean))
  ;[1 1 1] Only work with Non-UFocusable Objects
  (if (not bImplementsUFocusable)
    (bind _asprimitive_component (Utilities|Casting|CastToPrimitiveComponent Component))
    (Rendering|SetRenderCustomDepth _asprimitive_component bSelected)))

(event EventOnGizmoStateChanged
  (params (GizmoType :type ETransformationType%20Enum :default "TT_NoTransform") (bTransformInProgress :type Boolean) (Domain :type ETransformationDomain%20Enum :default "TD_None"))
  (CallFunction|ChangeInputeMode bTransformInProgress))

(event Input|ActionEvents|InputActionSelect
  (params (Key :type Key%20Structure :default "None"))
  ;[1 1 1] Select
  (:Pressed
    (Class|TransformerPawn|MouseTracebyObjectTypes (Variables|Default|GetTrace%20Distance) (Utilities|Array|MakeArray "ECC_GameTraceChannel1" "ECC_GameTraceChannel2") (Utilities|Array|MakeArray) false))
  (:Released
    (Class|TransformerPawn|ClearDomain)))

(event Input|AxisEvents|InputAxisMoveForward
  (params (AxisValue :type Float%20%28single-precision%29))
  (Transformation|AddActorWorldOffset (* (Transformation|GetActorForwardVector) (* AxisValue (Variables|Default|GetCameraMoveSpeed)))))

(event Input|AxisEvents|InputAxisMoveRight
  (params (AxisValue :type Float%20%28single-precision%29))
  (Transformation|AddActorWorldOffset (* (Transformation|GetActorRightVector) (* AxisValue (Variables|Default|GetCameraMoveSpeed)))))

(event Input|AxisEvents|InputAxisTurnRight
  (params (AxisValue :type Float%20%28single-precision%29))
  (Pawn|Input|AddControllerYawInput AxisValue))

(event Input|AxisEvents|InputAxisLookUp
  (params (AxisValue :type Float%20%28single-precision%29))
  (Pawn|Input|AddControllerPitchInput AxisValue))

(event Input|AxisEvents|InputAxisMoveUp
  (params (AxisValue :type Float%20%28single-precision%29))
  (Transformation|AddActorWorldOffset (Math|Vector|MakeVector 0.0 0.0 (* AxisValue (Variables|Default|GetCameraMoveSpeed)))))

(event Input|KeyboardEvents|Delete
  (params (Key :type Key%20Structure :default "None"))
  ;[1 1 1] Delete
  (:Pressed
    (Class|TransformerPawn|DeselectAll true)))

(event Input|KeyboardEvents|SpaceBar
  (params (Key :type Key%20Structure :default "None"))
  (:Pressed
    (CallFunction|ChangeTransformationType)))

(fn ConstructionScript)

(fn ChangeTransformationType
  (Class|TransformerPawn|SetTransformationType (select (Utilities|Enum|Equal(Enum) (Variables|Default|GetCurrentTransformation) "TT_Translation") "TT_Rotation" "TT_Translation"))
  (if (Utilities|Enum|Equal(Enum) (Variables|Default|GetCurrentTransformation) "TT_Translation")
    (Class|TransformerPawn|SetSpaceType "ST_World")
    (else
      (Class|TransformerPawn|SetSpaceType "ST_Local"))))

(fn ChangeInputeMode
  (params (TransformInProgress :type Boolean))
  (bind _asplayer_controller (Utilities|Casting|CastToPlayerController (Pawn|GetController)))
  (Input|SetInputModeGameandUI _asplayer_controller 0 (select TransformInProgress "LockAlways" "DoNotLock") (not TransformInProgress)))